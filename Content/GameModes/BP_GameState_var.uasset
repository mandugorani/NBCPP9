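; Game state for a two-player, turn-based match between Host and Guest, tracking a random number, the current turn and whether the game has ended.
; GameStart generates the number and clears the ended flag, while GameEnd sets it; both send debug text to every BP_Controller through GotBroadcast.
; SwitchTurn toggles the turn string.
; RepNotify handlers for all three variables only print debug messages.
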(event Custom|SwitchTurn
  (if (Utilities|Enum|Equal(Enum) (Variables|Default|GetTurn) "Host")
    (Variables|Default|SetTurn "Guest")
    (Development|PrintString "SwitchTurn : Guest !" true true "(R=0.000000,G=0.660000,B=1.000000,A=1.000000)" 22.0)
    (else
      (Variables|Default|SetTurn "Host")
      (Development|PrintString "SwitchTurn : Host !" true true "(R=0.000000,G=0.660000,B=1.000000,A=1.000000)" 22.0))))

(event Custom|GameStart
  (bind _returnvalue (Class|NumberBaseball|GenerateRandomNumber))
  (bind _output_get (Variables|Default|SetRandomNum _returnvalue))
  (bind _output_get_2 (Variables|Default|SetIsGameEnded false))
  (bind _outactors (Actor|GetAllActorsOfClass "/Script/Engine.PlayerController"))
  (for _array_element _outactors
    (bind _asbp_controller (Utilities|Casting|CastToBP_Controller _array_element))
    (Default|GotBroadcast _asbp_controller (Utilities|String|Append "Debug: currentRanNum: " _output_get "// Boolean_IsGameEnded: " (Utilities|String|ToString(Boolean) _output_get_2)))))

(event Custom|GameEnd
  (bind _output_get (Variables|Default|SetIsGameEnded true))
  (bind _outactors (Actor|GetAllActorsOfClass "/Script/Engine.PlayerController"))
  (for _array_element _outactors
    (bind _asbp_controller (Utilities|Casting|CastToBP_Controller _array_element))
    (Default|GotBroadcast _asbp_controller (Utilities|String|Append "IsGameEnded : " (Utilities|String|ToString(Boolean) _output_get)))))

(event EventBeginPlay)

(event EventTick
  (params (DeltaSeconds :type Float%20%28single-precision%29)))

(fn ConstructionScript)

(fn OnRepTurn
  (Development|PrintString (Utilities|String|Append "OnRep_Turn_Changed : " (Variables|Default|GetTurn))))

(fn OnRepIsGameEnded
  (Development|PrintString "OnRep_IsGameEnded_OK"))

(fn OnRepRandomNum
  (Development|PrintString "OnRep_RandomNum_OK"))